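; Tutorial component that tracks the current tutorial step and validates player actions against it.
; CheckTutorialFunction reports whether the tutorial is active and whether the passed step matches, pushing the step's "Wrong" text from TutorialTable on a mismatch.
; NextStep sets the step and shows its "Right" text.
; Messages go to every widget implementing In_TutorialUIControl, with rows looked up by enum name; debug prints log step changes.
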(fn `CheckTutorialFunction`
  (params (NewParam :type "/Game/BluePrint/Tables/TutorialStep Enum" :default "NewEnumerator0"))
  (returns (IsInTutorial :type Boolean) (IsRightButton :type Boolean))
  (`KismetSystemLibrary.PrintString` (`KismetStringLibrary.Concat_StrStr` (`|GetEnumeratorNameAsString` NewParam) "  check") true true (struct :`G` 0.66 :`B` 1.0 :`A` 1.0) 1.0)
  (`KismetSystemLibrary.PrintString` (`KismetStringLibrary.Concat_StrStr` (`|GetEnumeratorNameAsString` (`self.CurrentStep`)) " current check") true true (struct :`G` 0.66 :`B` 1.0 :`A` 1.0) 1.0)
  (if (`self.IsTutorial`)
    (if (`|EnumEquality` NewParam (`self.CurrentStep`))
      (return true true)
      (else
        (bind _foundwidgets (`WidgetBlueprintLibrary.GetAllWidgetsWithInterface` "/Game/BluePrint/Blueprints/Interface/In_TutorialUIControl.In_TutorialUIControl_C"))
        (for _array_element _foundwidgets
          (bind _returnvalue (`|GetDataTableRow` "/Game/BluePrint/Tables/TutorialTable.TutorialTable" (`KismetStringLibrary.Conv_StringToName` (`|GetEnumeratorNameAsString` (`self.CurrentStep`))))
            (:`then`
              (message `/Game/BluePrint/Blueprints/Interface/In_TutorialUIControl.Func_ChangeText` _array_element (`.wrong_9_8759306340D41105DBED4BB628FB832E` (break `/Game/BluePrint/Tables/TutorialStruct` _returnvalue)) "NewEnumerator0"))))
        (return true false)))
    (else
      (return false false))))

(fn `NextStep`
  (params (NewParam :type "/Game/BluePrint/Tables/TutorialStep Enum" :default "NewEnumerator0"))
  (bind _output_get (set `self.CurrentStep` NewParam))
  (`KismetSystemLibrary.PrintString` (`KismetStringLibrary.Concat_StrStr` (`|GetEnumeratorNameAsString` _output_get) " next") true true (struct :`G` 0.66 :`B` 1.0 :`A` 1.0) 1.0)
  (bind _foundwidgets (`WidgetBlueprintLibrary.GetAllWidgetsWithInterface` "/Game/BluePrint/Blueprints/Interface/In_TutorialUIControl.In_TutorialUIControl_C"))
  (for _array_element _foundwidgets
    (bind _returnvalue (`|GetDataTableRow` "/Game/BluePrint/Tables/TutorialTable.TutorialTable" (`KismetStringLibrary.Conv_StringToName` (`|GetEnumeratorNameAsString` (`self.CurrentStep`))))
      (:`then`
        (message `/Game/BluePrint/Blueprints/Interface/In_TutorialUIControl.Func_ChangeText` _array_element (`.right_8_18095F6C48D1E7BECE8248AED34C552B` (break `/Game/BluePrint/Tables/TutorialStruct` _returnvalue)) "NewEnumerator0")))))