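; Card distribution Blueprint that draws three distinct random cards to show to the player.
; CreateRandomZu builds weighted ordinary and rare pools from two data tables, repeating each card name by its Number.
; Random picks mostly from the ordinary pool, occasionally rare, matching names against the supplied card array until it has three unique entries.
; Each pick becomes a CardInformation object added to the MixtPawn's ShowCardBaseObject list.
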(event `Initialized Library`
  (bind _outrownames (`DataTableFunctionLibrary.GetDataTableRowNames` "/Game/BluePrint/Tables/OrdinaryCardRandom.OrdinaryCardRandom"))
  (for _array_element _outrownames
    (bind _returnvalue (`|GetDataTableRow` "/Game/BluePrint/Tables/OrdinaryCardRandom.OrdinaryCardRandom" _array_element)
      (:`then`
        (bind (_cardname _number) (break `/Game/BluePrint/Tables/CardDistribution` _returnvalue))
        (if (> _number (`self.AlreadyAdded`)) :!label _label
          (`KismetArrayLibrary.Array_Add` (`self.OrdinaryCardDistribution`) _cardname)
          (`/Engine/EditorBlueprintResources/StandardMacros.IncrementInt` (`self.AlreadyAdded`)
            (:`  `
              (goto _label)))
          (else
            (set `self.AlreadyAdded` 0))))))
  (bind _outrownames_2 (`DataTableFunctionLibrary.GetDataTableRowNames` "/Game/BluePrint/Tables/RareCardRandom.RareCardRandom"))
  (for _array_element_2 _outrownames_2
    (bind _returnvalue_2 (`|GetDataTableRow` "/Game/BluePrint/Tables/RareCardRandom.RareCardRandom" _array_element_2)
      (:`then`
        (bind (_cardname_2 _number_2) (break `/Game/BluePrint/Tables/CardDistribution` _returnvalue_2))
        (if (> _number_2 (`self.AlreadyAdded`)) :!label _label_2
          (`KismetArrayLibrary.Array_Add` (`self.RareCardDistribution`) _cardname_2)
          (`/Engine/EditorBlueprintResources/StandardMacros.IncrementInt` (`self.AlreadyAdded`)
            (:`  `
              (goto _label_2)))
          (else
            (set `self.AlreadyAdded` 0)))))))

(event `Random`
  (params (NewParam :type "Array of /Game/BluePrint/Blueprints/MainClasses/CardInformation Object Reference") (NewParam2 :type "Array of /Game/BluePrint/Tables/CardAttributes Structure"))
  (bind _temp_array1 (`self.Temp Array1`))
  (bind _temp_array1_2 (`self.Temp Array1`))
  (bind _asmixt_pawn (cast `/Game/BluePrint/Blueprints/MainClasses/MixtPawn` (`GameplayStatics.GetPlayerPawn` 0) :!pure true))
  (`KismetArrayLibrary.Array_Clear` NewParam)
  (`KismetArrayLibrary.Array_Clear` _temp_array1_2)
  (if (< (`KismetArrayLibrary.Array_Length` _temp_array1_2) 3) :!label _label_3
    (bind _output_get (set `self.NewVar_2` (`KismetMathLibrary.RandomInteger` 100)))
    (if (> _output_get 12)
      (set `self.NewVar_0` (`KismetArrayLibrary.Array_Random` (`self.OrdinaryCardDistribution`)))
      (else
        (set `self.NewVar_0` (`KismetArrayLibrary.Array_Random` (`self.RareCardDistribution`)))))
    (for _array_element NewParam2
      (if (== (`self.NewVar_0`) (`.Name_2_3E2EBFF54999AB25061B50B55136689D` (break `/Game/BluePrint/Tables/CardAttributes` _array_element)))
        (`KismetArrayLibrary.Array_AddUnique` _temp_array1 _array_element)))
    (goto _label_3)
    (else
      (for _array_element_2 _temp_array1
        (bind _returnvalue (`|GenericCreateObject` "/Game/BluePrint/Blueprints/MainClasses/CardInformation.CardInformation_C" _asmixt_pawn _array_element_2))
        (`KismetArrayLibrary.Array_AddUnique` (`/Game/BluePrint/Blueprints/MainClasses/MixtPawn.ShowCardBaseObject` _asmixt_pawn) _returnvalue)))))