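; MixtGameState is the game state that tracks the current turn and a shared CulturalPoint score.
; On BeginPlay it initializes each MixtPawn and its PlaceManager, then broadcasts turn 1 to all pawns.
; Rise adds points, copies the total to all pawns and plays a timed camera effect on player 0, which CulturalPoint's RepNotify also triggers.
; Turn advancement, game-end check and progress UI updates are disconnected.
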(event `Initial`
  (bind _outactors (`GameplayStatics.GetAllActorsOfClass` "/Game/BluePrint/Blueprints/MainClasses/MixtPawn.MixtPawn_C"))
  (for _array_element _outactors
    (`/Game/BluePrint/Blueprints/PlaceFunc/Func/PlaceManager.InitializeLevel` (`/Game/BluePrint/Blueprints/MainClasses/MixtPawn.PlaceManager` _array_element))
    (`/Game/BluePrint/Blueprints/MainClasses/MixtPawn.Initial` _array_element)))

(event `self.ReceiveBeginPlay`
  (`self.Initial`)
  (`self.NewTurn` 1))

(event `NewTurn`
  (params (NewParam :type Integer))
  (bind _output_get (set `self.CurrentGameTurn` NewParam))
  (bind _outactors (`GameplayStatics.GetAllActorsOfClass` "/Game/BluePrint/Blueprints/MainClasses/MixtPawn.MixtPawn_C"))
  (`KismetSystemLibrary.PrintString` (`KismetStringLibrary.Conv_IntToString` (`KismetArrayLibrary.Array_Length` _outactors)))
  (for _array_element _outactors
    (`/Game/BluePrint/Blueprints/MainClasses/MixtPawn.ChangeTurn` _array_element _output_get)))

(event `AddHeight`
  (params (NewParam :type Integer))
  (set `self.CulturalPoint` (+ (`self.CulturalPoint`) NewParam)))

(event `Rise`
  (params (value :type Integer))
  (bind _output_get (set `self.CulturalPoint` (+ (`self.CulturalPoint`) value)))
  (`|ExecutionSequence`
    (:`then_0`
      (bind _asmixt_pawn (cast `/Game/BluePrint/Blueprints/MainClasses/MixtPawn` (`GameplayStatics.GetPlayerPawn` 0)))
      (`/Game/BluePrint/Blueprints/MainClasses/MixtPawn.DriveCameraEffect` _asmixt_pawn _output_get)
      (`KismetSystemLibrary.Delay` 12.0)
      (bind _asmixt_pawn_2 (cast `/Game/BluePrint/Blueprints/MainClasses/MixtPawn` (`GameplayStatics.GetPlayerPawn` 0)))
      (`/Game/BluePrint/Blueprints/MainClasses/MixtPawn.BackToInCamera` _asmixt_pawn_2))
    (:`then_1`
      (bind _outactors (`GameplayStatics.GetAllActorsOfClass` "/Game/BluePrint/Blueprints/MainClasses/MixtPawn.MixtPawn_C"))
      (for _array_element _outactors
        (set `/Game/BluePrint/Blueprints/MainClasses/MixtPawn.CulturalPoint` (`self.CulturalPoint`) _array_element)))))

(fn `OnRep_CulturalPoint`
  (`KismetSystemLibrary.PrintString` "value change")
  (bind _asmixt_pawn (cast `/Game/BluePrint/Blueprints/MainClasses/MixtPawn` (`GameplayStatics.GetPlayerPawn` 0)))
  (`/Game/BluePrint/Blueprints/MainClasses/MixtPawn.DriveCameraEffect` _asmixt_pawn 0))

(fn `OnRep_CurrentEndNumber`)

(fn `OnRep_CurrentGameTurn`)

(fn `UserConstructionScript`)