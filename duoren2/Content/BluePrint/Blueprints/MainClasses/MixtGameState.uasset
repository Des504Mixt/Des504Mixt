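; MixtGameState is a game state Blueprint that runs a turn counter, starting the first turn on BeginPlay.
; NewTurn resets CurrentEndNumber and passes the current turn to player controller 0.
; RepNotifies drive the loop: reaching EndNumber increments the turn, which starts the next one or prints "Game ends" past MaxGameTurn.
; An unwired timeline would send cultural point progress toward Stage1Goal to the controller, but never runs.
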(event `self.ReceiveBeginPlay`
  (`self.NewTurn`))

(event `NewTurn`
  (set `self.CurrentEndNumber` 0)
  (bind _asmixt_player_controller (cast `/Game/BluePrint/Blueprints/MainClasses/MixtPlayerController` (`GameplayStatics.GetPlayerController` 0)))
  (`/Game/BluePrint/Blueprints/MainClasses/MixtPlayerController.ChangeTurn` _asmixt_player_controller (`self.CurrentGameTurn`)))

(fn `OnRep_CurrentEndNumber`
  (if (>= (`self.CurrentEndNumber`) (`self.EndNumber`))
    (set `self.CurrentGameTurn` (+ (`self.CurrentGameTurn`) 1))))

(fn `OnRep_CurrentGameTurn`
  (if (> (`self.CurrentGameTurn`) (`self.MaxGameTurn`))
    (`KismetSystemLibrary.PrintString` "Game ends")
    (else
      (`self.NewTurn`))))

(fn `UserConstructionScript`)