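; Player controller for a multiplayer, culture-themed card and building game with turns.
; Card, building, culture and turn calls mostly forward to MixtPawn; much of the controller's own version of that logic is left disconnected.
; Server events update MixtGameState, call MixtGameMode resets and decrement Scoreboard pools, with OnRep functions feeding personal counts to the Score widget.
; Remote instances show the menu on start and win screens when progress reaches 100%.
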(event `InputAxis|MoveForward`
  (params (AxisValue :type "Float (single-precision)"))
  ;[1 1 1] useless
)

(event `InputAxis|MoveRight`
  (params (AxisValue :type "Float (single-precision)"))
  ;[1 1 1] useless
)

(event `Recreate`
  (bind _returnvalue (`GameplayStatics.GetPlayerController` 0))
  (set `self.Finish` false)
  (set `self.Percentage` 0.0)
  (`/Engine/EditorBlueprintResources/ActorMacros.Switch Has Authority`
    (:`Remote`
      (`WidgetLayoutLibrary.RemoveAllWidgets`)
      (bind _returnvalue_2 (`|CreateWidget` "/Game/BluePrint/Blueprints/UI/TestUI/WBP_Menu.WBP_Menu_C" _returnvalue))
      (`UserWidget.AddToViewport` _returnvalue_2 0)
      (set `PlayerController.bShowMouseCursor` true _returnvalue))))

(event `AddBuilding`
  (params (card :type "/Game/BluePrint/Tables/CardAttributes Structure") (SectorType :type "/Game/BluePrint/Tables/SectorType Enum" :default "SectorType_MAX"))
  (bind _asmixt_pawn (cast `/Game/BluePrint/Blueprints/MainClasses/MixtPawn` (`GameplayStatics.GetPlayerPawn` 0)))
  (`/Game/BluePrint/Blueprints/MainClasses/MixtPawn.AddBuilding` _asmixt_pawn card SectorType))

(event `GetA`
  ;[1 1 1] useless
  (`/Engine/EditorBlueprintResources/ActorMacros.Switch Has Authority`
    (:`Remote`
      (`KismetSystemLibrary.PrintString` "Client")
      (`self.GetAServer`))))

(event `self.ReceiveBeginPlay`
  ;[1 1 1] Initial
  (`self.Recreate`))

(event `GetB`
  ;[1 1 1] useless
  (`/Engine/EditorBlueprintResources/ActorMacros.Switch Has Authority`
    (:`Remote`
      (`self.GetBServer`))))

(event `ChangeA`
  ;[1 1 1] useless
  (set `self.A` (+ (`self.A`) 1)))

(event `AddCultureBuildingServer`
  (params (NewParam :type "/Game/BluePrint/Tables/CardAttributes Structure"))
  (bind _asmixt_game_state (cast `/Game/BluePrint/Blueprints/MainClasses/MixtGameState` (`GameplayStatics.GetGameState`)))
  (`KismetArrayLibrary.Array_Add` (`/Game/BluePrint/Blueprints/MainClasses/MixtGameState.CulturalBuildings` _asmixt_game_state) NewParam)
  (set `/Game/BluePrint/Blueprints/MainClasses/MixtGameState.CulturalPoint` (+ (`.Output_46_4666DF0F4DEE94C12749D0BCDFDD14BC` (break `/Game/BluePrint/Tables/CardAttributes` NewParam)) (`/Game/BluePrint/Blueprints/MainClasses/MixtGameState.CulturalPoint` _asmixt_game_state)) _asmixt_game_state))

(event `ChangeB`
  ;[1 1 1] useless
  (set `self.B` (+ (`self.B`) 1)))

(event `PlayCardonServer`
  (params (card :type "/Game/BluePrint/Tables/CardAttributes Structure"))
  ;[1 1 1] PlayCard
)

(event `GetAServer`
  ;[1 1 1] useless
  (bind _returnvalue (`GameplayStatics.GetActorOfClass` "/Game/BluePrint/Blueprints/MainClasses/scoreboard.scoreboard_C"))
  (set `/Game/BluePrint/Blueprints/MainClasses/scoreboard.publicA` (- (`/Game/BluePrint/Blueprints/MainClasses/scoreboard.publicA` _returnvalue) 1) _returnvalue)
  (`self.ChangeA`))

(event `PlayCardLocal`
  (params (card :type "/Game/BluePrint/Tables/CardAttributes Structure"))
  ;[1 1 1] PlayCard
  (bind _asmixt_pawn (cast `/Game/BluePrint/Blueprints/MainClasses/MixtPawn` (`GameplayStatics.GetPlayerPawn` 0)))
  (`/Game/BluePrint/Blueprints/MainClasses/MixtPawn.PlayCardLocal` _asmixt_pawn card))

(event `GetBServer`
  ;[1 1 1] useless
  (bind _returnvalue (`GameplayStatics.GetActorOfClass` "/Game/BluePrint/Blueprints/MainClasses/scoreboard.scoreboard_C"))
  (set `/Game/BluePrint/Blueprints/MainClasses/scoreboard.publicB` (- (`/Game/BluePrint/Blueprints/MainClasses/scoreboard.publicB` _returnvalue) 1) _returnvalue)
  (`self.ChangeB`))

(event `AddCard`
  (params (NewParam :type "/Game/BluePrint/Tables/CardAttributes Structure"))
  (bind _asmixt_pawn (cast `/Game/BluePrint/Blueprints/MainClasses/MixtPawn` (`GameplayStatics.GetPlayerPawn` 0)))
  (`/Game/BluePrint/Blueprints/MainClasses/MixtPawn.AddCard` _asmixt_pawn NewParam))

(event `SelectCultureServer`
  (params (Culture :type "/Game/BluePrint/Tables/CultureType Enum" :default "NewEnumerator0"))
  ;[1 1 1] SelectCulture
  (`self.SelectCultureLocal` Culture))

(event `SelectCultureLocal`
  (params (NewParam :type "/Game/BluePrint/Tables/CultureType Enum" :default "NewEnumerator0"))
  ;[1 1 1] SelectCulture
  (bind _asmixt_pawn (cast `/Game/BluePrint/Blueprints/MainClasses/MixtPawn` (`GameplayStatics.GetPlayerPawn` 0)))
  (`/Game/BluePrint/Blueprints/MainClasses/MixtPawn.SelectCultureLocal` _asmixt_pawn NewParam))

(event `InitialCardBase`
  (params (Culture :type "/Game/BluePrint/Tables/CultureType Enum" :default "NewEnumerator0"))
  (bind _asmixt_pawn (cast `/Game/BluePrint/Blueprints/MainClasses/MixtPawn` (`GameplayStatics.GetPlayerPawn` 0)))
  ;[1 1 1] InitialCardBase
  (`/Game/BluePrint/Blueprints/MainClasses/MixtPawn.InitialCardBase` _asmixt_pawn Culture))

(event `EndTurnServer`
  ;[1 1 1] TurnRelated
  (bind _asmixt_game_state (cast `/Game/BluePrint/Blueprints/MainClasses/MixtGameState` (`GameplayStatics.GetGameState`)))
  (set `/Game/BluePrint/Blueprints/MainClasses/MixtGameState.CurrentEndNumber` (+ (`/Game/BluePrint/Blueprints/MainClasses/MixtGameState.CurrentEndNumber` _asmixt_game_state) 1) _asmixt_game_state)
  (`KismetSystemLibrary.PrintString` "end turn server"))

(event `EndTurnLocal`
  (bind _asmixt_pawn (cast `/Game/BluePrint/Blueprints/MainClasses/MixtPawn` (`GameplayStatics.GetPlayerPawn` 0)))
  (`/Game/BluePrint/Blueprints/MainClasses/MixtPawn.EndTurnLocal` _asmixt_pawn))

(event `ChangeTurn`
  (params (NewParam :type Integer))
  (bind _asmixt_pawn (cast `/Game/BluePrint/Blueprints/MainClasses/MixtPawn` (`GameplayStatics.GetPlayerPawn` 0)))
  ;[1 1 1] TurnRelated
  (`/Game/BluePrint/Blueprints/MainClasses/MixtPawn.ChangeTurn` _asmixt_pawn NewParam))

(event `PlaceBuilding`
  (params (NewParam :type "/Game/BluePrint/Tables/CardAttributes Structure")))

(event `GainOutput`
  (bind _asmixt_pawn (cast `/Game/BluePrint/Blueprints/MainClasses/MixtPawn` (`GameplayStatics.GetPlayerPawn` 0)))
  (`/Game/BluePrint/Blueprints/MainClasses/MixtPawn.GainOutput` _asmixt_pawn false))

(event `ChangePercentage`
  (params (Percentage :type "Float (double-precision)") (NewParam :type "Float (double-precision)") (NewParam2 :type "Float (double-precision)"))
  (bind _output_get (set `self.Percentage` (/ NewParam NewParam2)))
  (if (>= _output_get 1.0)
    (if (not (`self.Finish`))
      (set `self.Finish` true)
      (`/Engine/EditorBlueprintResources/ActorMacros.Switch Has Authority`
        (:`Remote`
          (`WidgetLayoutLibrary.RemoveAllWidgets`)
          (bind _returnvalue (`|CreateWidget` "/Game/BluePrint/Blueprints/UI/UsefulUI/WBP_Backtomenu.WBP_Backtomenu_C"))
          (`UserWidget.AddToViewport` _returnvalue 0)
          (bind _returnvalue_2 (`|CreateWidget` "/Game/BluePrint/Blueprints/UI/YouWin.YouWin_C"))
          (`UserWidget.AddToViewport` _returnvalue_2 0))))))

(event `ResetLevelServer`
  (`GameModeBase.ResetLevel` (`GameplayStatics.GetGameMode`))
  (`KismetSystemLibrary.PrintString` "reset"))

(event `RestartServer`
  (bind _asmixt_game_mode (cast `/Game/BluePrint/Blueprints/MainClasses/MixtGameMode` (`GameplayStatics.GetGameMode`)))
  (`/Game/BluePrint/Blueprints/MainClasses/MixtGameMode.RestartServer` _asmixt_game_mode))

(fn `BuyCard1`
  (params (NewParam :type "/Game/BluePrint/Tables/CardAttributes Structure"))
  (returns (NewParam1 :type Boolean))
  (bind _asmixt_pawn (cast `/Game/BluePrint/Blueprints/MainClasses/MixtPawn` (`GameplayStatics.GetPlayerPawn` 0)))
  (bind _newparam1 (`/Game/BluePrint/Blueprints/MainClasses/MixtPawn.BuyCard1` :`self` _asmixt_pawn))
  (return _newparam1))

(fn `OnRep_A`
  (bind _foundwidgets (`WidgetBlueprintLibrary.GetAllWidgetsOfClass` "/Game/BluePrint/Blueprints/MainClasses/Score.Score_C"))
  (set `/Game/BluePrint/Blueprints/MainClasses/Score.YourA` (`self.A`) (`|GetArrayItem` _foundwidgets)))

(fn `OnRep_B`
  (bind _foundwidgets (`WidgetBlueprintLibrary.GetAllWidgetsOfClass` "/Game/BluePrint/Blueprints/MainClasses/Score.Score_C"))
  (set `/Game/BluePrint/Blueprints/MainClasses/Score.YourB` (`self.B`) (`|GetArrayItem` _foundwidgets)))

(fn `RollDice`
  (locals (TempArray :type "Array of /Game/BluePrint/Tables/CardAttributes Structure"))
  (bind _showcardbaseobject (`self.ShowCardBaseObject`))
  (bind _temparray (`local.TempArray`))
  (`KismetArrayLibrary.Array_Clear` _showcardbaseobject)
  (if (< (`KismetArrayLibrary.Array_Length` _temparray) 5) :!label _label
    (`KismetArrayLibrary.Array_AddUnique` _temparray (`KismetArrayLibrary.Array_Random` (`self.CardBase`)))
    (goto _label)
    (else
      (`KismetSystemLibrary.PrintString` "Hello")
      (for _array_element _temparray
        (bind _returnvalue (`|GenericCreateObject` "/Game/BluePrint/Blueprints/MainClasses/CardInformation.CardInformation_C" self _array_element))
        (`KismetArrayLibrary.Array_AddUnique` _showcardbaseobject _returnvalue)))))

(fn `Show Hand Card`
  (returns (NewParam :type "Array of /Game/BluePrint/Blueprints/MainClasses/CardInformation Object Reference"))
  (bind _asmixt_pawn (cast `/Game/BluePrint/Blueprints/MainClasses/MixtPawn` (`GameplayStatics.GetPlayerPawn` 0)))
  (bind _newparam (`/Game/BluePrint/Blueprints/MainClasses/MixtPawn.ShowHandCard` _asmixt_pawn))
  (return _newparam))

(fn `ShowCardBase`
  (params (NewParam1 :type Integer))
  (returns (NewParam :type "Array of /Game/BluePrint/Blueprints/MainClasses/CardInformation Object Reference"))
  (locals (TempArray :type "Array of /Game/BluePrint/Tables/CardAttributes Structure"))
  (bind _asmixt_pawn (cast `/Game/BluePrint/Blueprints/MainClasses/MixtPawn` (`GameplayStatics.GetPlayerPawn` 0)))
  (return (`/Game/BluePrint/Blueprints/MainClasses/MixtPawn.ShowCardBaseObject` _asmixt_pawn)))

(fn `UserConstructionScript`)