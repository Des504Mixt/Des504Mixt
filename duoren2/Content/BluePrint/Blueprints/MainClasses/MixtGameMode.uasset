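; Server game mode for a turn-based, two-player Mixt match, handling turn flow, card hand-offs and restarts.
; RepNotify setters chain the flow: reaching the end count advances the turn, which either notifies every player controller or prints game over past the limit.
; Cards go to the other player's pawn, and restarts reset the level, shared state and players.
; The cultural-point progress broadcast is present but unconnected.
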(event `ClearAllObjects`
  (set `self.CurrentEndNumber` 0)
  (set `self.CurrentGameTurn` 0)
  (`KismetArrayLibrary.Array_Clear` (`self.CulturalBuildings`))
  (set `self.CulturalPoint` 0)
  (set `self.Percentage` 0.0))

(event `self.ReceiveBeginPlay`)

(event `RestartServer`
  (`self.ResetLevel`)
  (`self.ClearAllObjects`)
  (bind _returnvalue (`self.GetNumPlayers`))
  (for _index (range _returnvalue)
    (bind _returnvalue_2 (`GameplayStatics.GetPlayerController` _index))
    (`self.RestartPlayer` _returnvalue_2)
    (bind _asmixt_player_controller (cast `/Game/BluePrint/Blueprints/MainClasses/MixtPlayerController` _returnvalue_2))
    (`/Game/BluePrint/Blueprints/MainClasses/MixtPlayerController.Recreate` _asmixt_player_controller)))

(event `self.ReceiveTick`
  (params (DeltaSeconds :type "Float (single-precision)")))

(event `NewTurn`
  (set `self.CurrentEndNumber` 0)
  (bind _returnvalue (`self.GetNumPlayers`))
  (for _index (range _returnvalue)
    (bind _asmixt_player_controller (cast `/Game/BluePrint/Blueprints/MainClasses/MixtPlayerController` (`GameplayStatics.GetPlayerController` _index)))
    (`/Game/BluePrint/Blueprints/MainClasses/MixtPlayerController.ChangeTurn` _asmixt_player_controller (`self.CurrentGameTurn`))))

(event `GiveCardServer`
  (params (NewParam :type "/Game/BluePrint/Tables/CardAttributes Structure") (NewParam2 :type "PlayerController Object Reference"))
  (`KismetSystemLibrary.PrintString` "give card server")
  (if (== (`GameplayStatics.GetPlayerController` 0) NewParam2)
    (bind _asmixt_pawn (cast `/Game/BluePrint/Blueprints/MainClasses/MixtPawn` (`GameplayStatics.GetPlayerPawn` 1)))
    (`/Game/BluePrint/Blueprints/MainClasses/MixtPawn.ReceiveCard` _asmixt_pawn NewParam)
    (else
      (bind _asmixt_pawn_2 (cast `/Game/BluePrint/Blueprints/MainClasses/MixtPawn` (`GameplayStatics.GetPlayerPawn` 0)))
      (`/Game/BluePrint/Blueprints/MainClasses/MixtPawn.ReceiveCard` _asmixt_pawn_2 NewParam))))

(fn `OnRep_CurrentEndNumber`
  (if (>= (`self.CurrentEndNumber`) (`self.EndNumber`))
    (set `self.CurrentGameTurn` (+ (`self.CurrentGameTurn`) 1))))

(fn `OnRep_CurrentGameTurn`
  (if (> (`self.CurrentGameTurn`) (`self.MaxGameTurn`))
    (`KismetSystemLibrary.PrintString` "Game ends")
    (else
      (`self.NewTurn`))))

(fn `UserConstructionScript`)