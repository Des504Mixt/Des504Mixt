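; MixtPawn is the player pawn for a turn-based card building game, holding cards, Money, Human and action points.
; Culture choice loads a DataTable deck (or tutorial deck), from which RollDice offers three random cards as CardInformation objects.
; Played cards drive PlaceManager grid placement, then register by sector through MixtPlayerController.
; Turn ends increment a GameMode counter, while ChangeTurn applies income, refills actions and advances TutorialComponent steps.
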(event `InputAxis|MouseX`
  (params (AxisValue :type "Float (single-precision)")))

(event `InputAxis|MouseY`
  (params (AxisValue :type "Float (single-precision)")))

(event `InputAction|MouseUp`
  (params (Key :type "Key Structure")))

(event `InputAction|MouseDown`
  (params (Key :type "Key Structure")))

(event `PlaceBuildingPawn`
  (params (card :type "/Game/BluePrint/Tables/CardAttributes Structure"))
  (bind _placemanager (`self.PlaceManager`))
  (set `self.CurrentCard` card)
  (`self.DecreaseAction`)
  (set `self.CanRotate` false)
  (set `/Game/BluePrint/Blueprints/PlaceFunc/Func/PlaceManager.CurrentPlacingClass` "/Game/BluePrint/Blueprints/PlaceFunc/Buildings/Building_Example.Building_Example_C" _placemanager)
  (set `/Game/BluePrint/Blueprints/PlaceFunc/Func/PlaceManager.isPlacing` true _placemanager)
  (set `/Game/BluePrint/Blueprints/PlaceFunc/Func/PlaceManager.Spawned` false _placemanager))

(event `InputAction|AndytestStartPlace`
  (params (Key :type "Key Structure"))
  (bind _placemanager (`self.PlaceManager`))
  (:`Pressed`
    (set `/Game/BluePrint/Blueprints/PlaceFunc/Func/PlaceManager.isPlacing` true _placemanager)
    (set `/Game/BluePrint/Blueprints/PlaceFunc/Func/PlaceManager.Spawned` false _placemanager)))

(event `InitialSector`
  (bind _placemanager (`self.PlaceManager`))
  (bind _outactors (`GameplayStatics.GetAllActorsOfClass` "/Game/BluePrint/Blueprints/PlaceFunc/Func/GridInitializer.GridInitializer_C"))
  (for _array_element _outactors
    (bind _sectortype (`/Game/BluePrint/Blueprints/PlaceFunc/Func/GridInitializer.sectorType` _array_element))
    (if (== _sectortype "/Game/BluePrint/Blueprints/PlaceFunc/Func/BP_Grid_Blue.BP_Grid_Blue_C")
      (set `/Game/BluePrint/Blueprints/PlaceFunc/Func/PlaceManager.GridInitializer_Blue` _array_element _placemanager)
      (elif (== _sectortype "/Game/BluePrint/Blueprints/PlaceFunc/Func/BP_Grid_White.BP_Grid_White_C")
        (set `/Game/BluePrint/Blueprints/PlaceFunc/Func/PlaceManager.GridInitializer_White` _array_element _placemanager)
        (elif (== _sectortype "/Game/BluePrint/Blueprints/PlaceFunc/Func/BP_Grid_Green.BP_Grid_Green_C")
          (set `/Game/BluePrint/Blueprints/PlaceFunc/Func/PlaceManager.GridInitializer_Green` _array_element _placemanager)))))
  (`/Game/BluePrint/Blueprints/PlaceFunc/Func/PlaceManager.InitializeLevel` _placemanager))

(event `self.ReceiveBeginPlay`
  (bind _returnvalue (`GameplayStatics.GetPlayerController` 0))
  (set `PlayerController.bShowMouseCursor` true (`GameplayStatics.GetPlayerController` 0))
  (set `/Game/BluePrint/Blueprints/PlaceFunc/Func/PlaceManager.CurrentPlacingClass` "/Game/BluePrint/Blueprints/PlaceFunc/Buildings/Building_Example_2.Building_Example_2_C" (`self.PlaceManager`))
  (`/Engine/EditorBlueprintResources/ActorMacros.Switch Has Authority`
    (:`Remote`
      (`WidgetLayoutLibrary.RemoveAllWidgets`)
      (bind _returnvalue_2 (`|CreateWidget` "/Game/BluePrint/Blueprints/UI/TestUI/WBP_Menu.WBP_Menu_C" _returnvalue))
      (`UserWidget.AddToViewport` _returnvalue_2 0)
      (set `PlayerController.bShowMouseCursor` true _returnvalue)
      (`self.InitialSector`))))

(event `InputAction|AndytestPlace`
  (params (Key :type "Key Structure"))
  (bind _placemanager (`self.PlaceManager`))
  (:`Pressed`
    (if (`/Game/BluePrint/Blueprints/PlaceFunc/Buildings/Building_Parent.CanbePlaced` (`/Game/BluePrint/Blueprints/PlaceFunc/Func/PlaceManager.CurrentPlaceingObject` _placemanager))
      (set `/Game/BluePrint/Blueprints/PlaceFunc/Func/PlaceManager.Spawned` true _placemanager)
      (bind _asmixt_player_controller (cast `/Game/BluePrint/Blueprints/MainClasses/MixtPlayerController` (`GameplayStatics.GetPlayerController` 0)))
      (`/Game/BluePrint/Blueprints/MainClasses/MixtPlayerController.AddBuilding` _asmixt_player_controller (`self.CurrentCard`) (`self.CurrentSector`))
      (set `self.CurrentCard` (struct)))))

(event `InputAction|ＭouseLeft`
  (params (Key :type "Key Structure")))

(event `InitialCardBase`
  (params (Culture :type "/Game/BluePrint/Tables/CultureType Enum" :default "NewEnumerator0"))
  (bind _cardbase (`self.CardBase`))
  (bind _istutorial (`self.IsTutorial`))
  (bind _cardbase_2 (`self.CardBase`))
  ;[1 1 1] InitialCardBase
  (`KismetArrayLibrary.Array_Clear` (`self.CardBase`))
  (switch `/Game/BluePrint/Tables/CultureType` Culture
    (:`NewEnumerator0`
      (if _istutorial
        (bind _outrownames (`DataTableFunctionLibrary.GetDataTableRowNames` "/Game/BluePrint/Tables/TutorialCardBase.TutorialCardBase"))
        (for _array_element _outrownames
          (bind _returnvalue (`|GetDataTableRow` "/Game/BluePrint/Tables/TutorialCardBase.TutorialCardBase" _array_element)
            (:`then`
              (`KismetArrayLibrary.Array_Add` _cardbase _returnvalue)
              (for _array_element_2 _cardbase
                (setmembers `/Game/BluePrint/Tables/CardAttributes` :`StructRef` _array_element_2 :`CultureType` "NewEnumerator0")))))
        (else
          (bind _outrownames_2 (`DataTableFunctionLibrary.GetDataTableRowNames` "/Game/BluePrint/Tables/Chinese_card2.Chinese_card2"))
          (for _array_element_3 _outrownames_2
            (bind _returnvalue_2 (`|GetDataTableRow` "/Game/BluePrint/Tables/Chinese_card2.Chinese_card2" _array_element_3)
              (:`then`
                (`KismetArrayLibrary.Array_Add` (`self.CardBase`) _returnvalue_2)))))))
    (:`NewEnumerator1`
      (if _istutorial
        (bind _outrownames_3 (`DataTableFunctionLibrary.GetDataTableRowNames` "/Game/BluePrint/Tables/TutorialCardBase.TutorialCardBase"))
        (for _array_element_4 _outrownames_3
          (bind _returnvalue_3 (`|GetDataTableRow` "/Game/BluePrint/Tables/TutorialCardBase.TutorialCardBase" _array_element_4)
            (:`then`
              (`KismetArrayLibrary.Array_Add` _cardbase_2 _returnvalue_3)
              (for _array_element_5 _cardbase_2
                (setmembers `/Game/BluePrint/Tables/CardAttributes` :`StructRef` _array_element_5 :`CultureType` "NewEnumerator0")))))
        (else
          (bind _outrownames_4 (`DataTableFunctionLibrary.GetDataTableRowNames` "/Game/BluePrint/Tables/British_card_.British_card_"))
          (for _array_element_6 _outrownames_4
            (bind _returnvalue_4 (`|GetDataTableRow` "/Game/BluePrint/Tables/British_card_.British_card_" _array_element_6)
              (:`then`
                (`KismetArrayLibrary.Array_Add` (`self.CardBase`) _returnvalue_4)))))))))

(event `CostAction`)

(event `GainOutput`
  (params (IsCommercial :type Boolean))
  ;[1 1 1] GainOutputEachturn
  (if IsCommercial
    (set `self.MoneyGainPerTurn` 0)
    (for _array_element (`self.CommercialBuidings`)
      (set `self.MoneyGainPerTurn` (+ (`.Output_46_4666DF0F4DEE94C12749D0BCDFDD14BC` (break `/Game/BluePrint/Tables/CardAttributes` _array_element)) (`self.MoneyGainPerTurn`))))
    (else
      (set `self.HumanGainPerTurn` 0)
      (for _array_element_2 (`self.ResidentialBuildings`)
        (set `self.HumanGainPerTurn` (+ (`.Output_46_4666DF0F4DEE94C12749D0BCDFDD14BC` (break `/Game/BluePrint/Tables/CardAttributes` _array_element_2)) (`self.HumanGainPerTurn`)))
        (set `self.Human` (+ (`self.Human`) (`self.HumanGainPerTurn`)))))))

(event `GiveCard`
  (params (NewParam :type "/Game/BluePrint/Tables/CardAttributes Structure"))
  (`KismetSystemLibrary.PrintString` "give card in pawn")
  (bind _asmixt_game_mode (cast `/Game/BluePrint/Blueprints/MainClasses/MixtGameMode` (`GameplayStatics.GetGameMode`)))
  (`/Game/BluePrint/Blueprints/MainClasses/MixtGameMode.GiveCardServer` _asmixt_game_mode NewParam self))

(event `ReceiveCard`
  (params (NewParam :type "/Game/BluePrint/Tables/CardAttributes Structure"))
  (`KismetArrayLibrary.Array_Add` (`self.CardsOnHand`) NewParam)
  (`KismetSystemLibrary.PrintString` "receive card"))

(event `SelectCultureLocal`
  (params (NewParam :type "/Game/BluePrint/Tables/CultureType Enum" :default "NewEnumerator0"))
  (set `self.Culture` NewParam)
  (`self.InitialCardBase` NewParam)
  (`self.RollDice`))

(event `PlayCardLocal`
  (params (card :type "/Game/BluePrint/Tables/CardAttributes Structure"))
  (if (<= (`.HumanCost_11_08D3FB6144B331349B8C6C8C45DDA204` (break `/Game/BluePrint/Tables/CardAttributes` card)) (`self.Human`))
    (`self.PlaceBuildingPawn` card)))

(event `AddBuilding`
  (params (card :type "/Game/BluePrint/Tables/CardAttributes Structure") (SectorType :type "/Game/BluePrint/Tables/SectorType Enum" :default "SectorType_MAX"))
  ;[1 1 1] AddBuilding
  (`KismetArrayLibrary.Array_RemoveItem` (`self.CardsOnHand`) card)
  (bind _foundwidgets (`WidgetBlueprintLibrary.GetAllWidgetsWithInterface` "/Game/BluePrint/Blueprints/Interface/In_Confirm.In_Confirm_C"))
  (for _array_element _foundwidgets
    (message `/Game/BluePrint/Blueprints/Interface/In_Confirm.Func_Confirm` _array_element))
  (`|ExecutionSequence`
    (:`then_0`
      (switch `/Game/BluePrint/Tables/SectorType` SectorType
        (:`NewEnumerator0`
          (`KismetArrayLibrary.Array_Add` (`self.CommercialBuidings`) card))
        (:`NewEnumerator1`
          (`KismetArrayLibrary.Array_Add` (`self.ResidentialBuildings`) card))
        (:`NewEnumerator2`
          (bind _asmixt_player_controller (cast `/Game/BluePrint/Blueprints/MainClasses/MixtPlayerController` (`GameplayStatics.GetPlayerController` 0)))
          (`/Game/BluePrint/Blueprints/MainClasses/MixtPlayerController.AddCultureBuildingServer` _asmixt_player_controller card))))
    (:`then_1`
      (set `self.Human` (- (`self.Human`) (`.HumanCost_11_08D3FB6144B331349B8C6C8C45DDA204` (break `/Game/BluePrint/Tables/CardAttributes` card)))))))

(event `EndTurnServer`
  ;[1 1 1] TurnRelated
  (bind _asmixt_game_mode (cast `/Game/BluePrint/Blueprints/MainClasses/MixtGameMode` (`GameplayStatics.GetGameMode`)))
  (set `/Game/BluePrint/Blueprints/MainClasses/MixtGameMode.CurrentEndNumber` (+ (`/Game/BluePrint/Blueprints/MainClasses/MixtGameMode.CurrentEndNumber` _asmixt_game_mode) 1) _asmixt_game_mode)
  (`KismetSystemLibrary.PrintString` "end turn server"))

(event `EndTurnLocal`
  ;[1 1 1] TurnRelated
  (if (not (`self.IsEnd`))
    (set `self.IsEnd` true)
    (`self.RollDice`)
    (`self.EndTurnServer`)))

(event `ChangeTurn`
  (params (NewParam :type Integer))
  ;[1 1 1] TurnRelated
  (set `self.IsEnd` false)
  (set `self.TurnNumber` NewParam)
  (set `self.Money` (+ (`self.Money`) (`self.MoneyGainPerTurn`)))
  (set `self.Human` (+ (`self.Human`) (`self.HumanGainPerTurn`)))
  (set `self.ActionPoint` (`self.MaxActionPoint`))
  (if (`|EnumEquality` (`/Game/BluePrint/Blueprints/MainClasses/TutorialComponent.CurrentStep` (`self.TutorialComponent`)) "NewEnumerator5")
    (`/Game/BluePrint/Blueprints/MainClasses/TutorialComponent.NextStep` (`self.TutorialComponent`) "NewEnumerator6")
    (elif (`|EnumEquality` (`/Game/BluePrint/Blueprints/MainClasses/TutorialComponent.CurrentStep` (`self.TutorialComponent`)) "NewEnumerator14")
      (`/Game/BluePrint/Blueprints/MainClasses/TutorialComponent.NextStep` (`self.TutorialComponent`) "NewEnumerator7")
      (bind _foundwidgets (`WidgetBlueprintLibrary.GetAllWidgetsOfClass` "/Game/BluePrint/Blueprints/UI/UsefulUI/WBP_Bottombuttion.WBP_Bottombuttion_C"))
      (for _array_element _foundwidgets
        (set `/Game/BluePrint/Blueprints/UI/UsefulUI/WBP_Bottombuttion.Step` "NewEnumerator7" _array_element))
      (elif (`|EnumEquality` (`/Game/BluePrint/Blueprints/MainClasses/TutorialComponent.CurrentStep` (`self.TutorialComponent`)) "NewEnumerator15")
        (`/Game/BluePrint/Blueprints/MainClasses/TutorialComponent.NextStep` (`self.TutorialComponent`) "NewEnumerator29")
        (bind _foundwidgets_2 (`WidgetBlueprintLibrary.GetAllWidgetsOfClass` "/Game/BluePrint/Blueprints/UI/UsefulUI/WBP_Bottombuttion.WBP_Bottombuttion_C"))
        (for _array_element_2 _foundwidgets_2
          (set `/Game/BluePrint/Blueprints/UI/UsefulUI/WBP_Bottombuttion.Step_0` "NewEnumerator29" _array_element_2))
        (elif (`|EnumEquality` (`/Game/BluePrint/Blueprints/MainClasses/TutorialComponent.CurrentStep` (`self.TutorialComponent`)) "NewEnumerator19")
          (`/Game/BluePrint/Blueprints/MainClasses/TutorialComponent.NextStep` (`self.TutorialComponent`) "NewEnumerator20")
          (bind _foundwidgets_3 (`WidgetBlueprintLibrary.GetAllWidgetsOfClass` "/Game/BluePrint/Blueprints/UI/UsefulUI/WBP_Bottombuttion.WBP_Bottombuttion_C"))
          (for _array_element_3 _foundwidgets_3
            (set `/Game/BluePrint/Blueprints/UI/UsefulUI/WBP_Bottombuttion.Step` "NewEnumerator20" _array_element_3))
          (elif (`|EnumEquality` (`/Game/BluePrint/Blueprints/MainClasses/TutorialComponent.CurrentStep` (`self.TutorialComponent`)) "NewEnumerator24")
            (`/Game/BluePrint/Blueprints/MainClasses/TutorialComponent.NextStep` (`self.TutorialComponent`) "NewEnumerator23")
            (elif (`|EnumEquality` (`/Game/BluePrint/Blueprints/MainClasses/TutorialComponent.CurrentStep` (`self.TutorialComponent`)) "NewEnumerator31")
              (`/Game/BluePrint/Blueprints/MainClasses/TutorialComponent.NextStep` (`self.TutorialComponent`) "NewEnumerator28")
              (bind _foundwidgets_4 (`WidgetBlueprintLibrary.GetAllWidgetsOfClass` "/Game/BluePrint/Blueprints/UI/UsefulUI/WBP_Bottombuttion.WBP_Bottombuttion_C"))
              (for _array_element_4 _foundwidgets_4
                (set `/Game/BluePrint/Blueprints/UI/UsefulUI/WBP_Bottombuttion.Step_0` "NewEnumerator28" _array_element_4)))))))))

(event `AddCard`
  (params (NewParam :type "/Game/BluePrint/Tables/CardAttributes Structure"))
  ;[1 1 1] AddCard
  (`self.DecreaseAction`)
  (`KismetArrayLibrary.Array_Add` (`self.CardsOnHand`) NewParam)
  (bind _output_get (set `self.Money` (- (`self.Money`) (`.MoneyCost_13_6700F50D4F3D3C5183F8D0AE1FA1FBAA` (break `/Game/BluePrint/Tables/CardAttributes` NewParam)))))
  (`KismetSystemLibrary.PrintString` (`KismetStringLibrary.Conv_IntToString` _output_get))
  (`KismetSystemLibrary.PrintString` "add card controller"))

(fn `BuyCard1`
  (params (NewParam :type "/Game/BluePrint/Tables/CardAttributes Structure"))
  (returns (NewParam1 :type Boolean))
  (bind _newparam (`self.CheckAction`))
  (if _newparam
    (if (<= (`.MoneyCost_13_6700F50D4F3D3C5183F8D0AE1FA1FBAA` (break `/Game/BluePrint/Tables/CardAttributes` NewParam)) (`self.Money`))
      (`KismetSystemLibrary.PrintString` "chekc true")
      (return true)
      (else
        (return false)))
    (else
      (return false))))

(fn `CheckAction`
  (returns (NewParam :type Boolean))
  (if (> (`self.ActionPoint`) 0)
    (return true)
    (else
      (return false))))

(fn `DecreaseAction`
  (set `self.ActionPoint` (- (`self.ActionPoint`) 1)))

(fn `PlaceCard`
  (params (NewParam1 :type "/Game/BluePrint/Tables/CardAttributes Structure"))
  (returns (NewParam :type Boolean))
  (bind _newparam (`self.CheckAction`))
  (if _newparam
    (if (<= (`.HumanCost_11_08D3FB6144B331349B8C6C8C45DDA204` (break `/Game/BluePrint/Tables/CardAttributes` NewParam1)) (`self.Human`))
      (`KismetSystemLibrary.PrintString` "Place")
      (`self.PlaceBuildingPawn` NewParam1)
      (return true)
      (else
        (return false)))
    (else
      (return false))))

(fn `RollDice`
  (locals (TempArray :type "Array of /Game/BluePrint/Tables/CardAttributes Structure"))
  (bind _showcardbaseobject (`self.ShowCardBaseObject`))
  (bind _temparray (`local.TempArray`))
  (`KismetArrayLibrary.Array_Clear` _showcardbaseobject)
  (if (< (`KismetArrayLibrary.Array_Length` _temparray) 3) :!label _label
    (`KismetArrayLibrary.Array_AddUnique` _temparray (`KismetArrayLibrary.Array_Random` (`self.CardBase`)))
    (goto _label)
    (else
      (`KismetSystemLibrary.PrintString` "Hello")
      (for _array_element _temparray
        (bind _returnvalue (`|GenericCreateObject` "/Game/BluePrint/Blueprints/MainClasses/CardInformation.CardInformation_C" self _array_element))
        (`KismetArrayLibrary.Array_AddUnique` _showcardbaseobject _returnvalue)))))

(fn `ShowCardBase`
  (params (NewParam1 :type Integer))
  (returns (NewParam :type "Array of /Game/BluePrint/Blueprints/MainClasses/CardInformation Object Reference"))
  (locals (TempArray :type "Array of /Game/BluePrint/Tables/CardAttributes Structure"))
  (return (`self.ShowCardBaseObject`)))

(fn `ShowHandCard`
  (returns (NewParam :type "Array of /Game/BluePrint/Blueprints/MainClasses/CardInformation Object Reference"))
  (bind _cardonhandobject (`self.CardOnhandObject`))
  (`KismetArrayLibrary.Array_Clear` _cardonhandobject)
  (for _array_element (`self.CardsOnHand`)
    (bind _returnvalue (`|GenericCreateObject` "/Game/BluePrint/Blueprints/MainClasses/CardInformation.CardInformation_C" self _array_element))
    (`KismetArrayLibrary.Array_Add` _cardonhandobject _returnvalue))
  (return _cardonhandobject))

(fn `UserConstructionScript`)