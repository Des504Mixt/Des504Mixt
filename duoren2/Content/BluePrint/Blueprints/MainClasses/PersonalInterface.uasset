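; PersonalInterface is an actor Blueprint that manages UI widgets and opens the culture selection screen at BeginPlay.
; Its Initial event creates and stores the MainView, CardList and CultureSelection widgets.
; ShowMenu and QuitMenu add a given widget to the viewport or remove it.
; All three events act only on the Remote branch of an authority switch, so the UI runs only where the actor lacks authority.
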(event `ShowMenu`
  (params (Widget :type "UserWidget Object Reference"))
  (`/Engine/EditorBlueprintResources/ActorMacros.Switch Has Authority`
    (:`Remote`
      (`UserWidget.AddToViewport` Widget 0))))

(event `self.ReceiveBeginPlay`
  (`self.Initial`)
  (`self.ShowMenu` (`self.CultureSelection`)))

(event `QuitMenu`
  (params (Widget :type "UserWidget Object Reference"))
  (`/Engine/EditorBlueprintResources/ActorMacros.Switch Has Authority`
    (:`Remote`
      (`Widget.RemoveFromParent` Widget))))

(event `Initial`
  (`/Engine/EditorBlueprintResources/ActorMacros.Switch Has Authority`
    (:`Remote`
      (bind _returnvalue (`|CreateWidget` "/Game/BluePrint/Blueprints/UI/MainView.MainView_C"))
      (set `self.MainView` _returnvalue)
      (bind _returnvalue_2 (`|CreateWidget` "/Game/BluePrint/Blueprints/UI/CardList.CardList_C"))
      (set `self.CardList` _returnvalue_2)
      (bind _returnvalue_3 (`|CreateWidget` "/Game/BluePrint/Blueprints/UI/CultureSelection.CultureSelection_C"))
      (set `self.CultureSelection` _returnvalue_3))))

(fn `UserConstructionScript`)