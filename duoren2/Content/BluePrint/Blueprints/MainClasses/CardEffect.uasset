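; Card effect handler that applies China and UK culture card abilities to the player's MixtPawn resources and buildings.
; PlayCardFire dispatches Effects A, C and D and ActivateFire dispatches Effect B, both switching on the card's culture and effect.
; A and B add Human for China or Money for UK.
; C boosts the first opposite-culture building's output via DoOnce and D boosts all of them, residential or commercial depending on culture.
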(event `ActivateFire`
  (params (CardAttribue :type "/Game/BluePrint/Tables/CardAttributes Structure") (PlacedSector :type Boolean))
  (bind (_name _wheretoplace _culturetype _humancost _moneycost _humanoutput _moneyoutput _cultureoutput _specialeffect) (break `/Game/BluePrint/Tables/CardAttributes` CardAttribue))
  (bind _asmixt_pawn (cast `/Game/BluePrint/Blueprints/MainClasses/MixtPawn` (`GameplayStatics.GetPlayerPawn` 0) :!pure true))
  (bind _asmixt_pawn_2 (cast `/Game/BluePrint/Blueprints/MainClasses/MixtPawn` (`GameplayStatics.GetPlayerPawn` 0) :!pure true))
  (switch `/Game/BluePrint/Tables/CultureType` _culturetype
    (:`NewEnumerator0`
      (switch `/Game/BluePrint/Tables/SpecialEffect` _specialeffect
        (:`NewEnumerator1`
          (set `/Game/BluePrint/Blueprints/MainClasses/MixtPawn.Human` (+ (`/Game/BluePrint/Blueprints/MainClasses/MixtPawn.Human` _asmixt_pawn) 1) _asmixt_pawn))))
    (:`NewEnumerator1`
      (switch `/Game/BluePrint/Tables/SpecialEffect` _specialeffect
        (:`NewEnumerator1`
          (set `/Game/BluePrint/Blueprints/MainClasses/MixtPawn.Money` (+ (`/Game/BluePrint/Blueprints/MainClasses/MixtPawn.Money` _asmixt_pawn_2) 1) _asmixt_pawn_2))))))

(event `Hybrid`)

(event `PlayCardFire`
  (params (CardAttribue :type "/Game/BluePrint/Tables/CardAttributes Structure") (PlacedSector :type Boolean))
  (bind (_name _wheretoplace _culturetype _humancost _moneycost _humanoutput _moneyoutput _cultureoutput _specialeffect) (break `/Game/BluePrint/Tables/CardAttributes` CardAttribue))
  (bind _asmixt_pawn (cast `/Game/BluePrint/Blueprints/MainClasses/MixtPawn` (`GameplayStatics.GetPlayerPawn` 0) :!pure true))
  (bind _asmixt_pawn_2 (cast `/Game/BluePrint/Blueprints/MainClasses/MixtPawn` (`GameplayStatics.GetPlayerPawn` 0) :!pure true))
  (switch `/Game/BluePrint/Tables/CultureType` _culturetype
    (:`NewEnumerator0`
      (switch `/Game/BluePrint/Tables/SpecialEffect` _specialeffect
        (:`NewEnumerator0`
          (set `/Game/BluePrint/Blueprints/MainClasses/MixtPawn.Human` (+ (`/Game/BluePrint/Blueprints/MainClasses/MixtPawn.Human` _asmixt_pawn) 2) _asmixt_pawn))
        (:`NewEnumerator2`
          (for (_array_element _array_index) (`/Game/BluePrint/Blueprints/MainClasses/MixtPawn.ResidentialBuildings` (cast `/Game/BluePrint/Blueprints/MainClasses/MixtPawn` (`GameplayStatics.GetPlayerPawn` 0) :!pure true))
            (bind (_name_2 _wheretoplace_2 _culturetype_2 _humancost_2 _moneycost_2 _humanoutput_2) (break `/Game/BluePrint/Tables/CardAttributes` _array_element))
            (switch `/Game/BluePrint/Tables/CultureType` _culturetype_2
              (:`NewEnumerator1`
                (`/Engine/EditorBlueprintResources/StandardMacros.DoOnce` false :!label _label
                  (:`Completed`
                    (bind _structout (setmembers `/Game/BluePrint/Tables/CardAttributes` :`StructRef` _array_element :`HumanOutput` (+ _humanoutput_2 2)))
                    (`KismetArrayLibrary.Array_Set` (`/Game/BluePrint/Blueprints/MainClasses/MixtPawn.ResidentialBuildings` (cast `/Game/BluePrint/Blueprints/MainClasses/MixtPawn` (`GameplayStatics.GetPlayerPawn` 0) :!pure true)) _array_index _structout)
                    (`KismetSystemLibrary.PrintString` "FireC"))))))
          (goto _label :!via `Reset`))
        (:`NewEnumerator3`
          (for (_array_element_2 _array_index_2) (`/Game/BluePrint/Blueprints/MainClasses/MixtPawn.CommercialBuidings` (cast `/Game/BluePrint/Blueprints/MainClasses/MixtPawn` (`GameplayStatics.GetPlayerPawn` 0) :!pure true))
            (bind (_name_3 _wheretoplace_3 _culturetype_3 _humancost_3 _moneycost_3 _humanoutput_3 _moneyoutput_2) (break `/Game/BluePrint/Tables/CardAttributes` _array_element_2))
            (switch `/Game/BluePrint/Tables/CultureType` _culturetype_3
              (:`NewEnumerator1`
                (bind _structout_2 (setmembers `/Game/BluePrint/Tables/CardAttributes` :`StructRef` _array_element_2 :`MoneyOutput` (+ _moneyoutput_2 1)))
                (`KismetArrayLibrary.Array_Set` (`/Game/BluePrint/Blueprints/MainClasses/MixtPawn.CommercialBuidings` (cast `/Game/BluePrint/Blueprints/MainClasses/MixtPawn` (`GameplayStatics.GetPlayerPawn` 0) :!pure true)) _array_index_2 _structout_2)
                (`KismetSystemLibrary.PrintString` "FIreD")))))))
    (:`NewEnumerator1`
      (switch `/Game/BluePrint/Tables/SpecialEffect` _specialeffect
        (:`NewEnumerator0`
          (set `/Game/BluePrint/Blueprints/MainClasses/MixtPawn.Money` (+ (`/Game/BluePrint/Blueprints/MainClasses/MixtPawn.Money` _asmixt_pawn_2) 2) _asmixt_pawn_2))
        (:`NewEnumerator2`
          (for (_array_element_3 _array_index_3) (`/Game/BluePrint/Blueprints/MainClasses/MixtPawn.CommercialBuidings` (cast `/Game/BluePrint/Blueprints/MainClasses/MixtPawn` (`GameplayStatics.GetPlayerPawn` 0) :!pure true))
            (bind (_name_4 _wheretoplace_4 _culturetype_4 _humancost_4 _moneycost_4 _humanoutput_4 _moneyoutput_3) (break `/Game/BluePrint/Tables/CardAttributes` _array_element_3))
            (switch `/Game/BluePrint/Tables/CultureType` _culturetype_4
              (:`NewEnumerator0`
                (`/Engine/EditorBlueprintResources/StandardMacros.DoOnce` false :!label _label_2
                  (:`Completed`
                    (bind _structout_3 (setmembers `/Game/BluePrint/Tables/CardAttributes` :`StructRef` _array_element_3 :`MoneyOutput` (+ _moneyoutput_3 2)))
                    (`KismetArrayLibrary.Array_Set` (`/Game/BluePrint/Blueprints/MainClasses/MixtPawn.CommercialBuidings` (cast `/Game/BluePrint/Blueprints/MainClasses/MixtPawn` (`GameplayStatics.GetPlayerPawn` 0) :!pure true)) _array_index_3 _structout_3)
                    (`KismetSystemLibrary.PrintString` "FireC"))))))
          (goto _label_2 :!via `Reset`))
        (:`NewEnumerator3`
          (for (_array_element_4 _array_index_4) (`/Game/BluePrint/Blueprints/MainClasses/MixtPawn.ResidentialBuildings` (cast `/Game/BluePrint/Blueprints/MainClasses/MixtPawn` (`GameplayStatics.GetPlayerPawn` 0) :!pure true))
            (bind (_name_5 _wheretoplace_5 _culturetype_5 _humancost_5 _moneycost_5 _humanoutput_5) (break `/Game/BluePrint/Tables/CardAttributes` _array_element_4))
            (switch `/Game/BluePrint/Tables/CultureType` _culturetype_5
              (:`NewEnumerator0`
                (bind _structout_4 (setmembers `/Game/BluePrint/Tables/CardAttributes` :`StructRef` _array_element_4 :`HumanOutput` (+ _humanoutput_5 1)))
                (`KismetArrayLibrary.Array_Set` (`/Game/BluePrint/Blueprints/MainClasses/MixtPawn.ResidentialBuildings` (cast `/Game/BluePrint/Blueprints/MainClasses/MixtPawn` (`GameplayStatics.GetPlayerPawn` 0) :!pure true)) _array_index_4 _structout_4)
                (`KismetSystemLibrary.PrintString` "FIreD")))))))))

(fn `新函数_0`)