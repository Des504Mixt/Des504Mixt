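; Scoreboard Blueprint that mirrors two replicated values, PublicA and PublicB, into the on-screen Score widget.
; BeginPlay copies both values into the first top-level Score widget it finds.
; RepNotify functions, gated to Remote by SwitchHasAuthority, look up that widget again and push the changed value, with OnRep_score updating PublicA and OnRep_publicB updating PublicB.
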(event `self.ReceiveBeginPlay`
  (bind _foundwidgets (`WidgetBlueprintLibrary.GetAllWidgetsOfClass` "/Game/BluePrint/Blueprints/Score.Score_C"))
  (bind _output (`|GetArrayItem` _foundwidgets))
  (set `/Game/BluePrint/Blueprints/Score.publicA` (`self.publicA`) _output)
  (set `/Game/BluePrint/Blueprints/Score.publicB` (`self.publicB`) _output))

(fn `OnRep_publicB`
  (`/Engine/EditorBlueprintResources/ActorMacros.Switch Has Authority`
    (:`Remote`
      (bind _foundwidgets (`WidgetBlueprintLibrary.GetAllWidgetsOfClass` "/Game/BluePrint/Blueprints/Score.Score_C"))
      (set `/Game/BluePrint/Blueprints/Score.publicB` (`self.publicB`) (`|GetArrayItem` _foundwidgets)))))

(fn `OnRep_score`
  (`/Engine/EditorBlueprintResources/ActorMacros.Switch Has Authority`
    (:`Remote`
      (bind _foundwidgets (`WidgetBlueprintLibrary.GetAllWidgetsOfClass` "/Game/BluePrint/Blueprints/Score.Score_C"))
      (set `/Game/BluePrint/Blueprints/Score.publicA` (`self.publicA`) (`|GetArrayItem` _foundwidgets)))))

(fn `UserConstructionScript`)