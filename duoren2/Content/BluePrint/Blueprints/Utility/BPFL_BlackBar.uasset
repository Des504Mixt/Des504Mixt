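; Blueprint function library that shows and dismisses a black bar fade overlay through the BlackFadeUI widget.
; StartFade creates the widget for player 0, adds it to the viewport and plays its BlackBarOpen animation.
; EndFade takes the first top-level BlackFadeUI found, plays that animation in reverse and binds a delegate to its completion.
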(fn `EndFade`
  (bind _foundwidgets (`WidgetBlueprintLibrary.GetAllWidgetsOfClass` null "/Game/UI/BlackFadeUI.BlackFadeUI_C"))
  (bind _output (`|GetArrayItem` _foundwidgets))
  (bind _blackbaropen (`/Game/UI/BlackFadeUI.BlackBarOpen` _output))
  (`UserWidget.PlayAnimation` _output _blackbaropen 0.0 1 "Reverse" 1.0 false)
  (`UserWidget.BindToAnimationFinished` _output _blackbaropen (`|CreateDelegate` _output :!event `RemoveFromParent`)))

(fn `StartFade`
  (locals (BalckBarUI :type "/Game/UI/BlackFadeUI Object Reference"))
  (bind _balckbarui (`local.BalckBarUI`))
  (bind _returnvalue (`|CreateWidget` "/Game/UI/BlackFadeUI.BlackFadeUI_C" (`GameplayStatics.GetPlayerController` null)))
  (bind _output_get (set `local.BalckBarUI` _returnvalue))
  (`UserWidget.AddToViewport` _output_get 0)
  (`UserWidget.PlayAnimation` _balckbarui (`/Game/UI/BlackFadeUI.BlackBarOpen` _balckbarui) 0.0 1 "Forward" 1.0 false))