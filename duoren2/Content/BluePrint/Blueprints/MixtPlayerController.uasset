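; Multiplayer player controller that lets a client take units of two resources, A and B, from a shared Scoreboard actor into its own counts.
; GetA and GetB act only on the Remote branch, calling server-named events that decrement the Scoreboard's public count, without a bounds check, and increment the controller's.
; RepNotify functions copy A and B to the first Score widget.
; Movement and look input logic is left unconnected.
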(event `InputAxis|MoveForward`
  (params (AxisValue :type "Float (single-precision)")))

(event `InputAxis|MoveRight`
  (params (AxisValue :type "Float (single-precision)")))

(event `InputAxis|Turn` :overrideparent false
  (params (AxisValue :type "Float (single-precision)")))

(event `InputAxis|LookUp` :overrideparent false
  (params (AxisValue :type "Float (single-precision)")))

(event `InputAction|decrease`
  (params (Key :type "Key Structure")))

(event `GetA`
  (`/Engine/EditorBlueprintResources/ActorMacros.Switch Has Authority`
    (:`Remote`
      (`KismetSystemLibrary.PrintString` "Client")
      (`self.GetAServer`))))

(event `GetB`
  (`/Engine/EditorBlueprintResources/ActorMacros.Switch Has Authority`
    (:`Remote`
      (`self.GetBServer`))))

(event `GetAServer`
  (bind _returnvalue (`GameplayStatics.GetActorOfClass` "/Game/BluePrint/Blueprints/scoreboard.scoreboard_C"))
  (set `/Game/BluePrint/Blueprints/scoreboard.publicA` (- (`/Game/BluePrint/Blueprints/scoreboard.publicA` _returnvalue) 1) _returnvalue)
  (`self.ChangeA`))

(event `ChangeA`
  (set `self.A` (+ (`self.A`) 1)))

(event `GetBServer`
  (bind _returnvalue (`GameplayStatics.GetActorOfClass` "/Game/BluePrint/Blueprints/scoreboard.scoreboard_C"))
  (set `/Game/BluePrint/Blueprints/scoreboard.publicB` (- (`/Game/BluePrint/Blueprints/scoreboard.publicB` _returnvalue) 1) _returnvalue)
  (`self.ChangeB`))

(event `ChangeB`
  (set `self.B` (+ (`self.B`) 1)))

(fn `OnRep_A`
  (bind _foundwidgets (`WidgetBlueprintLibrary.GetAllWidgetsOfClass` "/Game/BluePrint/Blueprints/Score.Score_C"))
  (set `/Game/BluePrint/Blueprints/Score.YourA` (`self.A`) (`|GetArrayItem` _foundwidgets)))

(fn `OnRep_B`
  (bind _foundwidgets (`WidgetBlueprintLibrary.GetAllWidgetsOfClass` "/Game/BluePrint/Blueprints/Score.Score_C"))
  (set `/Game/BluePrint/Blueprints/Score.YourB` (`self.B`) (`|GetArrayItem` _foundwidgets)))

(fn `UserConstructionScript`)