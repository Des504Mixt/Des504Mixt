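; PersonalSector is a player-controlled pawn Blueprint that handles mouse-driven orbit and zoom for a spring-arm camera.
; Horizontal mouse input adds controller yaw, while vertical input sets the control rotation directly, clamping pitch between looking straight ahead and steeply downward.
; MouseUp and MouseDown actions play and reverse a single timeline that drives the SpringArm's length, moving smoothly along one zoom curve.
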(event `InputAxis|MouseX`
  (params (AxisValue :type "Float (single-precision)"))
  (`self.AddControllerYawInput` AxisValue))

(event `InputAxis|MouseY`
  (params (AxisValue :type "Float (single-precision)"))
  (`Controller.SetControlRotation` (`GameplayStatics.GetPlayerController` 0) (`KismetMathLibrary.MakeRotator` (.roll (`self.GetControlRotation`)) (`KismetMathLibrary.ClampAngle` (+ AxisValue (.pitch (`self.GetControlRotation`))) -70.0) (.yaw (`self.GetControlRotation`)))))

(event `InputAction|MouseUp`
  (params (Key :type "Key Structure"))
  (:`Pressed`
    (bind (_direction _newtrack_0) (`Timeline|Timeline_0` :!label _label)
      (:`Update`
        (set `SpringArmComponent.TargetArmLength` _newtrack_0 (`self.SpringArm`))))))

(event `InputAction|MouseDown`
  (params (Key :type "Key Structure"))
  (:`Pressed`
    (goto _label :!via `Reverse`)))

(fn `UserConstructionScript`)